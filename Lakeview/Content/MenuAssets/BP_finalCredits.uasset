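; Final credits actor that scrolls through the level by moving itself, then closes the game.
; BeginPlay starts two parallel timers: a short delay sets a flag that starts the scroll, and a three-minute delay, timed to the song, quits the game.
; While the flag is set, Tick adds the DeltaS offset to the actor's location each frame, with no frame-time scaling shown.
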(event EventTick
  (params (DeltaSeconds :type Float%20%28single-precision%29))
  ;[1 1 1] Final Credits Scroll Down
  (if (Variables|Default|Getwait10sec)
    (Transformation|SetActorLocation (+ (Transformation|GetActorLocation) (Variables|Default|GetDeltaS)) false false)))

(event EventBeginPlay
  (Utilities|FlowControl|Sequence
    (:then_0
      ;[1 1 1] Final Credits Scroll Down
      (Utilities|FlowControl|Delay 1e+01)
      (Variables|Default|Setwait10sec true))
    (:then_1
      ;[1 1 1] Quit Game after the song
      (Utilities|FlowControl|Delay 1.8e+02)
      (Development|PrintString "End of the Game")
      (Game|QuitGame 0 "Quit" false))))

(fn ConstructionScript)